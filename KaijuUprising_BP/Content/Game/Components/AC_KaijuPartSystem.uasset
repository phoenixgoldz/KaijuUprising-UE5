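; Actor component that tracks per-part health on a kaiju and derives its total health from the parts.
; Initialization refills every part, and damage by part type clamps that part's health, re-sums the total and returns whether a break occurred.
; A part reaching zero while not flagged broken records its loot material ID and spawns a Niagara damage effect.
; Query functions return unbroken parts and collected loot IDs.
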(event EventBeginPlay)

(event EventTick
  (params (DeltaSeconds :type Float%20%28single-precision%29)))

(fn InitializeBodyParts
  (bind _bodyparts (Variables|Default|GetBodyParts))
  (Variables|Default|SetTotalHealth 0.0)
  (for _index (range 0 (- (Utilities|Array|Length (Variables|Default|GetBodyParts)) 1))
    (Utilities|Array|SetArrayElem _bodyparts _index (Utilities|Struct|MakeS_KaijuBodyPart (.PartType (Utilities|Struct|BreakS_KaijuBodyPart (Utilities|Array|Get(acopy) _bodyparts _index))) (.PartName (Utilities|Struct|BreakS_KaijuBodyPart (Utilities|Array|Get(acopy) _bodyparts _index))) (.MaxHealth (Utilities|Struct|BreakS_KaijuBodyPart (Utilities|Array|Get(acopy) _bodyparts _index))) (.MaxHealth (Utilities|Struct|BreakS_KaijuBodyPart (Utilities|Array|Get(acopy) _bodyparts _index))) (.BreakThreshold (Utilities|Struct|BreakS_KaijuBodyPart (Utilities|Array|Get(acopy) _bodyparts _index))) (.IsBroken (Utilities|Struct|BreakS_KaijuBodyPart (Utilities|Array|Get(acopy) _bodyparts _index))) (.CollisionComponent (Utilities|Struct|BreakS_KaijuBodyPart (Utilities|Array|Get(acopy) _bodyparts _index))) (.LootMaterialID (Utilities|Struct|BreakS_KaijuBodyPart (Utilities|Array|Get(acopy) _bodyparts _index)))))
    (Variables|Default|SetTotalHealth (+ (Variables|Default|GetTotalHealth) (.MaxHealth (Utilities|Struct|BreakS_KaijuBodyPart (Utilities|Array|Get(acopy) _bodyparts _index))))))
  (Variables|Default|SetCurrentTotalHealth (Variables|Default|GetTotalHealth)))

(fn DamageBodyPart
  (params (PartType :type E_KaijuPartType%20Enum :default "NewEnumerator0") (Damage :type Float%20%28single-precision%29))
  (bind _bodyparts (Variables|Default|GetBodyParts))
  (Utilities|FlowControl|Sequence
    (:then_0
      (Variables|Default|SetFoundIndex -1)
      (Variables|Default|SetPartBrokenFlag false)
      (for _index (range 0 (- (Utilities|Array|Length _bodyparts) 1))
        (if (Utilities|Enum|Equal(Enum) (.PartType (Utilities|Struct|BreakS_KaijuBodyPart (Utilities|Array|Get(acopy) _bodyparts _index))) PartType)
          (Variables|Default|SetFoundIndex _index)))
      (if (>= (Variables|Default|GetFoundIndex) 0)
        (Variables|Default|SetNewHealth (select (> (select (< (- (.CurrentHealth (Utilities|Struct|BreakS_KaijuBodyPart (Utilities|Array|Get(acopy) (Variables|Default|GetBodyParts) (Variables|Default|GetFoundIndex)))) Damage) 0.0) 0.0 (- (.CurrentHealth (Utilities|Struct|BreakS_KaijuBodyPart (Utilities|Array|Get(acopy) (Variables|Default|GetBodyParts) (Variables|Default|GetFoundIndex)))) Damage)) (.MaxHealth (Utilities|Struct|BreakS_KaijuBodyPart (Utilities|Array|Get(acopy) (Variables|Default|GetBodyParts) (Variables|Default|GetFoundIndex))))) (.MaxHealth (Utilities|Struct|BreakS_KaijuBodyPart (Utilities|Array|Get(acopy) (Variables|Default|GetBodyParts) (Variables|Default|GetFoundIndex)))) (select (< (- (.CurrentHealth (Utilities|Struct|BreakS_KaijuBodyPart (Utilities|Array|Get(acopy) (Variables|Default|GetBodyParts) (Variables|Default|GetFoundIndex)))) Damage) 0.0) 0.0 (- (.CurrentHealth (Utilities|Struct|BreakS_KaijuBodyPart (Utilities|Array|Get(acopy) (Variables|Default|GetBodyParts) (Variables|Default|GetFoundIndex)))) Damage))))
        (if (and (== (select (> (select (< (- (.CurrentHealth (Utilities|Struct|BreakS_KaijuBodyPart (Utilities|Array|Get(acopy) (Variables|Default|GetBodyParts) (Variables|Default|GetFoundIndex)))) Damage) 0.0) 0.0 (- (.CurrentHealth (Utilities|Struct|BreakS_KaijuBodyPart (Utilities|Array|Get(acopy) (Variables|Default|GetBodyParts) (Variables|Default|GetFoundIndex)))) Damage)) (.MaxHealth (Utilities|Struct|BreakS_KaijuBodyPart (Utilities|Array|Get(acopy) (Variables|Default|GetBodyParts) (Variables|Default|GetFoundIndex))))) (.MaxHealth (Utilities|Struct|BreakS_KaijuBodyPart (Utilities|Array|Get(acopy) (Variables|Default|GetBodyParts) (Variables|Default|GetFoundIndex)))) (select (< (- (.CurrentHealth (Utilities|Struct|BreakS_KaijuBodyPart (Utilities|Array|Get(acopy) (Variables|Default|GetBodyParts) (Variables|Default|GetFoundIndex)))) Damage) 0.0) 0.0 (- (.CurrentHealth (Utilities|Struct|BreakS_KaijuBodyPart (Utilities|Array|Get(acopy) (Variables|Default|GetBodyParts) (Variables|Default|GetFoundIndex)))) Damage))) 0.0) (not (.IsBroken (Utilities|Struct|BreakS_KaijuBodyPart (Utilities|Array|Get(acopy) (Variables|Default|GetBodyParts) (Variables|Default|GetFoundIndex))))))
          (Variables|Default|SetPartBrokenFlag true)
          (Utilities|Array|Add (Variables|Default|GetBrokenParts) (.LootMaterialID (Utilities|Struct|BreakS_KaijuBodyPart (Utilities|Array|Get(acopy) (Variables|Default|GetBodyParts) (Variables|Default|GetFoundIndex)))))
          (Niagara|SpawnSystematLocation (.CollisionComponent (Utilities|Struct|BreakS_KaijuBodyPart (Utilities|Array|Get(acopy) (Variables|Default|GetBodyParts) (Variables|Default|GetFoundIndex)))) "/Game/Variant_Combat/VFX/NS_Damage.NS_Damage" (Transformation|GetWorldLocation (.CollisionComponent (Utilities|Struct|BreakS_KaijuBodyPart (Utilities|Array|Get(acopy) (Variables|Default|GetBodyParts) (Variables|Default|GetFoundIndex))))))
          (Utilities|Array|SetArrayElem (Variables|Default|GetBodyParts) (Variables|Default|GetFoundIndex) (Utilities|Struct|MakeS_KaijuBodyPart (.PartType (Utilities|Struct|BreakS_KaijuBodyPart (Utilities|Array|Get(acopy) (Variables|Default|GetBodyParts) (Variables|Default|GetFoundIndex)))) (.PartName (Utilities|Struct|BreakS_KaijuBodyPart (Utilities|Array|Get(acopy) (Variables|Default|GetBodyParts) (Variables|Default|GetFoundIndex)))) (.MaxHealth (Utilities|Struct|BreakS_KaijuBodyPart (Utilities|Array|Get(acopy) (Variables|Default|GetBodyParts) (Variables|Default|GetFoundIndex)))) (Variables|Default|GetNewHealth) (.BreakThreshold (Utilities|Struct|BreakS_KaijuBodyPart (Utilities|Array|Get(acopy) (Variables|Default|GetBodyParts) (Variables|Default|GetFoundIndex)))) true (.CollisionComponent (Utilities|Struct|BreakS_KaijuBodyPart (Utilities|Array|Get(acopy) (Variables|Default|GetBodyParts) (Variables|Default|GetFoundIndex)))) (.LootMaterialID (Utilities|Struct|BreakS_KaijuBodyPart (Utilities|Array|Get(acopy) (Variables|Default|GetBodyParts) (Variables|Default|GetFoundIndex))))))
          (else
            (Utilities|Array|SetArrayElem (Variables|Default|GetBodyParts) (Variables|Default|GetFoundIndex) (Utilities|Struct|MakeS_KaijuBodyPart (.PartType (Utilities|Struct|BreakS_KaijuBodyPart (Utilities|Array|Get(acopy) (Variables|Default|GetBodyParts) (Variables|Default|GetFoundIndex)))) (.PartName (Utilities|Struct|BreakS_KaijuBodyPart (Utilities|Array|Get(acopy) (Variables|Default|GetBodyParts) (Variables|Default|GetFoundIndex)))) (.MaxHealth (Utilities|Struct|BreakS_KaijuBodyPart (Utilities|Array|Get(acopy) (Variables|Default|GetBodyParts) (Variables|Default|GetFoundIndex)))) (Variables|Default|GetNewHealth) (.BreakThreshold (Utilities|Struct|BreakS_KaijuBodyPart (Utilities|Array|Get(acopy) (Variables|Default|GetBodyParts) (Variables|Default|GetFoundIndex)))) (.IsBroken (Utilities|Struct|BreakS_KaijuBodyPart (Utilities|Array|Get(acopy) (Variables|Default|GetBodyParts) (Variables|Default|GetFoundIndex)))) (.CollisionComponent (Utilities|Struct|BreakS_KaijuBodyPart (Utilities|Array|Get(acopy) (Variables|Default|GetBodyParts) (Variables|Default|GetFoundIndex)))) (.LootMaterialID (Utilities|Struct|BreakS_KaijuBodyPart (Utilities|Array|Get(acopy) (Variables|Default|GetBodyParts) (Variables|Default|GetFoundIndex))))))))))
    (:then_1
      (Variables|Default|SetTotalHealthSum 0.0)
      (for _array_element (Variables|Default|GetBodyParts)
        (Variables|Default|SetTotalHealthSum (+ (Variables|Default|GetTotalHealthSum) (.CurrentHealth (Utilities|Struct|BreakS_KaijuBodyPart _array_element)))))
      (Variables|Default|SetCurrentTotalHealth (Variables|Default|GetTotalHealthSum))
      (return (Variables|Default|GetPartBrokenFlag)))))

(fn GetTargetableParts
  (bind _array (Utilities|Array|MakeArray ""))
  (for _array_element (Variables|Default|GetBodyParts)
    (if (not (.IsBroken (Utilities|Struct|BreakS_KaijuBodyPart _array_element)))
      (Utilities|Array|Add _array _array_element)))
  (return _array))

(fn GetBrokenPartLoot
  (return (Variables|Default|GetBrokenParts)))